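; BP_AG_Basket is a basket that checks whether objects are delivered in a requested order.
; When an actor begins overlapping its Box, it loops through that actor's GrabComponents and ignores any that are held.
; An ObjectType matching the current ObjectAsked entry prints a debug message and advances ObjectAskedNumber to the next request.
; The check runs only at overlap start, with no bounds check on the index.
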(event `self.Box.OnComponentBeginOverlap`
  (params (OverlappedComponent :type "PrimitiveComponent Object Reference") (OtherActor :type "Actor Object Reference") (OtherComp :type "PrimitiveComponent Object Reference") (OtherBodyIndex :type Integer) (bFromSweep :type Boolean) (SweepResult :type "HitResult Structure (by ref)"))
  (bind _returnvalue (`self.K2_GetComponentsByClass` OtherActor "/Game/TemplateFolder/VRTemplate/Blueprints/GrabComponent.GrabComponent_C"))
  (`KismetSystemLibrary.PrintString` "Contact")
  (if (> (`KismetArrayLibrary.Array_Length` _returnvalue) 0)
    (for _array_element _returnvalue
      (if (`/Game/TemplateFolder/VRTemplate/Blueprints/GrabComponent.bIsHeld` _array_element)
        _
        (elif (`|EnumEquality` (`/Game/TemplateFolder/VRTemplate/Blueprints/GrabComponent.ObjectType` _array_element) (`|GetArrayItem` (`self.Object Asked`) (`self.ObjectAskedNumber`)))
          (`KismetSystemLibrary.PrintString` "Gut")
          (`/Engine/EditorBlueprintResources/StandardMacros.IncrementInt` (`self.ObjectAskedNumber`)))))))

(fn `UserConstructionScript`)