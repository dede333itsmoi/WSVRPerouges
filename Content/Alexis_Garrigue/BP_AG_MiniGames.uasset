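; Base actor for VR mini-game entry points that yaw toward the player's headset on a looping timer.
; When hit, it hides its capsule, plays a fade sequence, moves the pawn to the game location with teleporting disabled, and reveals the game's objects.
; EndMiniGame plays effects, fades, returns the pawn and restores the world.
; GameMaster handles tree changes and world visibility; MiniGame is an empty hook for game logic.
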(event `self.ReceiveBeginPlay`
  (`KismetSystemLibrary.K2_SetTimerDelegate` (delegate `LookPlayer`) 0.1 true))

(event `LookPlayer`
  (bind (_returnvalue_roll _returnvalue_pitch) (`KismetMathLibrary.BreakRotator` (`self.K2_GetActorRotation`)))
  (bind _asbp_ag_vrpawn (cast `/Game/Alexis_Garrigue/BP_AG_VRPawn` (`GameplayStatics.GetPlayerPawn` 0)))
  (bind (_returnvalue_roll_2 _returnvalue_pitch_2 _returnvalue_yaw) (`KismetMathLibrary.BreakRotator` (`KismetMathLibrary.FindLookAtRotation` (`self.K2_GetActorLocation`) (`SceneComponent.K2_GetComponentLocation` (`/Game/Alexis_Garrigue/BP_AG_VRPawn.HeadMountedDisplayMesh` _asbp_ag_vrpawn)))))
  (`self.K2_SetActorRotation` (`KismetMathLibrary.MakeRotator` _returnvalue_roll _returnvalue_pitch _returnvalue_yaw)))

(event `Hit`
  (bind _capsule (`self.Capsule`))
  (`PrimitiveComponent.SetCollisionEnabled` _capsule "NoCollision")
  (`SceneComponent.SetVisibility` _capsule false false)
  (`self.StartMiniGame`))

(event `StartMiniGame`
  (`/Game/Alexis_Garrigue/BP_AG_GameMaster.HideAll` (`self.GameMaster`))
  (bind _asbp_ag_vrpawn (cast `/Game/Alexis_Garrigue/BP_AG_VRPawn` (`GameplayStatics.GetPlayerPawn` 0)))
  (bind _returnvalue (`GameplayStatics.GetActorOfClass` "/Script/LevelSequence.LevelSequenceActor"))
  (`LevelSequenceActor.SetSequence` _returnvalue "/Game/Cesar/BP/LS_CVC_LongFade.LS_CVC_LongFade")
  (`MovieSceneSequencePlayer.Play` (`LevelSequenceActor.SequencePlayer` _returnvalue))
  (`KismetSystemLibrary.Delay` 0.75)
  (`/Game/Alexis_Garrigue/BP_AG_GameMaster.ChangeTree` (`self.GameMaster`) (`self.TreeNumber`))
  (`self.K2_SetActorLocation` _asbp_ag_vrpawn (`self.K2_GetActorLocation` (`self.GameLocation`)) false false)
  (`self.MiniGame`)
  (set `/Game/Alexis_Garrigue/BP_AG_VRPawn.CanTeleport` false _asbp_ag_vrpawn)
  (for _array_element (`self.ObjectsInGame`)
    (`/Engine/EditorBlueprintResources/StandardMacros.IsValid` _array_element
      (:`Is Valid`
        (`self.SetActorHiddenInGame` _array_element false)))))

(event `EndMiniGame`
  (bind _capsule (`self.Capsule`))
  (bind _gamemaster (`self.GameMaster`))
  (`GameplayStatics.PlaySound2D` null 1.0 1.0 0.0 null null)
  (bind _returnvalue (`AddComponent|NODE_AddNiagaraComponent-1` :`self` (`self.GameMaster`)))
  (`NiagaraFunctionLibrary.SpawnSystemAttached` "/Game/Cesar/VFX/N_CVC_Smok1.N_CVC_Smok1" _returnvalue "None" (`self.Location`) (struct) "KeepRelativeOffset")
  (`KismetSystemLibrary.Delay` 3.0)
  (bind _asbp_ag_vrpawn (cast `/Game/Alexis_Garrigue/BP_AG_VRPawn` (`GameplayStatics.GetPlayerPawn` 0)))
  (bind _returnvalue_2 (`GameplayStatics.GetActorOfClass` "/Script/LevelSequence.LevelSequenceActor"))
  (`LevelSequenceActor.SetSequence` _returnvalue_2 "/Game/Cesar/BP/LS_CVC_LongFade.LS_CVC_LongFade")
  (`MovieSceneSequencePlayer.Play` (`LevelSequenceActor.SequencePlayer` _returnvalue_2))
  (`KismetSystemLibrary.Delay` 0.75)
  (`/Game/Alexis_Garrigue/BP_AG_GameMaster.ChangeTree` _gamemaster 0)
  (bind _returnvalue_3 (`AddComponent|NODE_AddNiagaraComponent-3` :`self` _gamemaster))
  (`NiagaraFunctionLibrary.SpawnSystemAttached` "/Game/Cesar/VFX/N_CVC_ExploArbre.N_CVC_ExploArbre" _returnvalue_3 "bite" (0.0 -50.0 50.0) (struct) "KeepRelativeOffset")
  (`self.K2_SetActorLocation` _asbp_ag_vrpawn (`self.K2_GetActorLocation` (`self.TPLocation`)) false false)
  (`PrimitiveComponent.SetCollisionEnabled` _capsule "QueryOnly")
  (`SceneComponent.SetVisibility` _capsule true false)
  (set `/Game/Alexis_Garrigue/BP_AG_VRPawn.CanTeleport` true _asbp_ag_vrpawn)
  (for _array_element (`self.ObjectsInGame`)
    (`/Engine/EditorBlueprintResources/StandardMacros.IsValid` _array_element
      (:`Is Valid`
        (`self.SetActorHiddenInGame` _array_element true))))
  (`/Game/Alexis_Garrigue/BP_AG_GameMaster.ShowAll` (`self.GameMaster`)))

(fn `MiniGame`)

(fn `UserConstructionScript`)