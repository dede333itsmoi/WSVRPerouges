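; BP_AG_Kayoo is a block object that can lock itself in place and register with a Wall.
; Locking starts a one-shot timer of TimeForLock that fires Counter.
; If IsIn is still true when the timer fires, Counter disables physics simulation on the static mesh and passes the block to the Wall through AddBlock.
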(event `Locking`
  (bind _returnvalue (`KismetSystemLibrary.K2_SetTimerDelegate` (delegate `Counter`) (`self.TimeForLock`)))
  (set `self.Timer` _returnvalue))

(event `Counter`
  (if (`self.IsIn`)
    (`PrimitiveComponent.SetSimulatePhysics` (`self.StaticMesh`) false)
    (`/Game/Alexis_Garrigue/Wall/BP_AG_WallTrigger.AddBlock` (`self.Wall`) self)))

(fn `UserConstructionScript`
  (`parent.UserConstructionScript`))