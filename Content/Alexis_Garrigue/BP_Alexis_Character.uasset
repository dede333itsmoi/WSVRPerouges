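; VR player character that sets up stage tracking and hand input contexts when a headset is enabled, and teleports between placed BP_Alexis_TpPoint actors.
; Holding the search input runs a looping timer that line-traces from the right aim controller and prints any teleport point hit.
; The teleport input repeats the trace and moves the character to that point.
; Both traces end at the scaled forward vector, without adding the controller's location.
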(event `self.ReceiveBeginPlay`
  (bind _returnvalue (pcsubsystem `EnhancedInputLocalPlayerSubsystem` (`GameplayStatics.GetPlayerController` 0)))
  (if (`HeadMountedDisplayFunctionLibrary.IsHeadMountedDisplayEnabled`)
    (`HeadMountedDisplayFunctionLibrary.SetTrackingOrigin` "Stage")
    (`KismetSystemLibrary.ExecuteConsoleCommand` "vr.PixelDensity 1.0" null)
    (`EnhancedInputSubsystemInterface.AddMappingContext` _returnvalue "/Game/TemplateFolder/VRTemplate/Input/IMC_Default.IMC_Default" 0 (struct))
    (`EnhancedInputSubsystemInterface.AddMappingContext` _returnvalue "/Game/TemplateFolder/VRTemplate/Input/IMC_Hands.IMC_Hands" 0 (struct))))

(event `InputAction|Searching for Tp`
  (params (Key :type "Key Structure"))
  (:`Pressed`
    (bind _returnvalue (`KismetSystemLibrary.K2_SetTimerDelegate` (delegate `Tp Search`) 0.1 true))
    (set `self.TpSearchLoop` _returnvalue))
  (:`Released`
    (`KismetSystemLibrary.K2_ClearAndInvalidateTimerHandle` (`self.TpSearchLoop`))))

(event `Tp Search`
  (`self.Searching For Tp`))

(event `InputAction|Teleport`
  (params (Key :type "Key Structure"))
  (bind _motioncontrollerrightaim (`self.MotionControllerRightAim`))
  (:`Pressed`
    (bind _outhit (`KismetSystemLibrary.LineTraceSingle` (`SceneComponent.K2_GetComponentLocation` _motioncontrollerrightaim) (* (`SceneComponent.GetForwardVector` _motioncontrollerrightaim) 1000.0) "TraceTypeQuery1"))
    (bind _asbp_alexis_tp_point (cast `/Game/Alexis_Garrigue/BP_Alexis_TpPoint` (`.HitActor` (`GameplayStatics.BreakHitResult` _outhit))))
    (`self.K2_SetActorLocation` (`self.K2_GetActorLocation` _asbp_alexis_tp_point))))

(fn `Searching For Tp`
  (bind _motioncontrollerrightaim (`self.MotionControllerRightAim`))
  (bind _outhit (`KismetSystemLibrary.LineTraceSingle` (`SceneComponent.K2_GetComponentLocation` _motioncontrollerrightaim) (* (`SceneComponent.GetForwardVector` _motioncontrollerrightaim) 1000.0) "TraceTypeQuery1"))
  (bind _asbp_alexis_tp_point (cast `/Game/Alexis_Garrigue/BP_Alexis_TpPoint` (`.HitActor` (`GameplayStatics.BreakHitResult` _outhit))))
  (`KismetSystemLibrary.PrintString` (`KismetSystemLibrary.GetDisplayName` _asbp_alexis_tp_point)))

(fn `UserConstructionScript`)