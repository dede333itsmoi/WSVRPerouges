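; Wall trigger actor for a mini-game that collects objects entering its box and ends once five overlaps are recorded.
; Each overlapping actor is added to the Placed array, and any BP_AG_Object has physics simulation switched off on its mesh.
; At the threshold, the trigger moves to a hardcoded location and re-enables physics on the placed objects.
; The count includes any overlapping actor, as adding happens before the cast.
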(event `self.Box.OnComponentBeginOverlap`
  (params (OverlappedComponent :type "PrimitiveComponent Object Reference") (OtherActor :type "Actor Object Reference") (OtherComp :type "PrimitiveComponent Object Reference") (OtherBodyIndex :type Integer) (bFromSweep :type Boolean) (SweepResult :type "HitResult Structure (by ref)"))
  (`KismetArrayLibrary.Array_Add` (`self.Placed`) OtherActor)
  (bind _asbp_ag_object (cast `/Game/Alexis_Garrigue/Objects/BP_AG_Object` OtherActor))
  (`PrimitiveComponent.SetSimulatePhysics` (`/Game/Alexis_Garrigue/Objects/BP_AG_Object.StaticMesh` _asbp_ag_object) false)
  (if (>= (`KismetArrayLibrary.Array_Length` (`self.Placed`)) 5)
    (`self.EndOfMiniGame`)))

(event `EndOfMiniGame`
  (`self.K2_SetActorLocation` (70.0 1770.0 180.0))
  (for _array_element (`self.Placed`)
    (bind _asbp_ag_object (cast `/Game/Alexis_Garrigue/Objects/BP_AG_Object` _array_element))
    (`PrimitiveComponent.SetSimulatePhysics` (`/Game/Alexis_Garrigue/Objects/BP_AG_Object.StaticMesh` _asbp_ag_object) true)))

(fn `UserConstructionScript`)