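; BP_AG_WallGame is the wall-building minigame about the 1468 siege, where debris from a demolished house is stacked against a gate.
; MiniGame resets the Wall, then runs timed French narration, subtitles and quest text through GameMaster.
; SpawnKayoo swaps the House for effects and ten scattered BP_AG_Kayoo debris actors with meshes taken from Ruins.
; A Blocker volume blocks collision briefly during the spawn, then the stacking quest is set.
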(event `SpawnKayoo`
  (bind _house (`self.House`))
  (bind (_houseloc_x _houseloc_y) (`KismetMathLibrary.BreakVector` (`self.HouseLoc`)))
  (bind _ruins (`self.Ruins`))
  (bind (_returnvalue_x _returnvalue_y _returnvalue_z) (`KismetMathLibrary.BreakVector` (`self.K2_GetActorLocation` (`self.House`))))
  (`NiagaraFunctionLibrary.SpawnSystemAtLocation` "/Game/Cesar/VFX/N_CVC_aled.N_CVC_aled" (`KismetMathLibrary.MakeVector` _returnvalue_x _returnvalue_y (+ _returnvalue_z 100.0)))
  (`GameplayStatics.PlaySound2D` "/Game/Cesar/SFX/WallBreakReduced.WallBreakReduced" 0.2 1.0 0.0 null null)
  (set `self.HouseLoc` (`SceneComponent.K2_GetComponentLocation` (`/Game/Alexis_Garrigue/Wall/BP_AG_House.Arrow` _house)))
  (`self.K2_DestroyActor` _house)
  (`PrimitiveComponent.SetCollisionResponseToAllChannels` (`Brush.BrushComponent` (`self.Blocker`)) "ECR_Block")
  (for _index (range 10)
    (bind _returnvalue (`|SpawnActorFromClass` "/Game/Alexis_Garrigue/Objects/BP_AG_Kayoo.BP_AG_Kayoo_C" (`KismetMathLibrary.MakeTransform` (`KismetMathLibrary.MakeVector` (+ _houseloc_x (`KismetMathLibrary.RandomFloatInRange` -70.0 70.0)) (+ _houseloc_y (`KismetMathLibrary.RandomFloatInRange` -70.0 70.0)) 700.0) (struct) (2.0 2.0 2.0)) "Undefined" "MultiplyWithRoot" null null))
    (`StaticMeshComponent.SetStaticMesh` (`/Game/Alexis_Garrigue/Objects/BP_AG_Object.StaticMesh` _returnvalue) (`|GetArrayItem` _ruins _index))
    (`KismetArrayLibrary.Array_Remove` _ruins _index))
  (`KismetSystemLibrary.Delay` 0.5)
  (`PrimitiveComponent.SetCollisionResponseToAllChannels` (`Brush.BrushComponent` (`self.Blocker`)) "ECR_Ignore")
  (`/Game/Alexis_Garrigue/BP_AG_GameMaster.Quest` (`self.GameMaster`) "- Ramasses les débris et empiles les contre la porte. "))

(event `BeginningDialogue`
  (bind _gamemaster (`self.GameMaster`))
  (bind _returnvalue (`self.K2_GetActorLocation` _gamemaster))
  (`GameplayStatics.PlaySoundAtLocation` "/Game/Alexis_Garrigue/Dialogues/A_DebutSiegeAttaque.A_DebutSiegeAttaque" _returnvalue (struct) 1.0 1.0 0.0 null null null null)
  (`/Game/Alexis_Garrigue/BP_AG_GameMaster.Subtitles` _gamemaster "1468, les Dauphinois du royaume de France attaquent la cité alors Savoyarde.")
  (`KismetSystemLibrary.Delay` 7.2)
  (`GameplayStatics.PlaySoundAtLocation` "/Game/Alexis_Garrigue/Dialogues/A_SiegeBravesPerougiens.A_SiegeBravesPerougiens" _returnvalue (struct) 1.0 1.0 0.0 null null null null)
  (`/Game/Alexis_Garrigue/BP_AG_GameMaster.Subtitles` _gamemaster "Ils s’en prennent à la Porte du Bas, moins défendue.")
  (`KismetSystemLibrary.Delay` 3.0)
  (`/Game/Alexis_Garrigue/BP_AG_GameMaster.Subtitles` _gamemaster "Mais les braves et ingénieux pérougiens")
  (`KismetSystemLibrary.Delay` 4.0)
  (`/Game/Alexis_Garrigue/BP_AG_GameMaster.Subtitles` _gamemaster "utilisent les pierres de la ville pour y bâtir un mur en une nuit.")
  (`KismetSystemLibrary.Delay` 3.0)
  (`GameplayStatics.PlaySoundAtLocation` "/Game/Alexis_Garrigue/Dialogues/A_SiegeDevoirConstruire.A_SiegeDevoirConstruire" _returnvalue (struct) 1.0 1.0 0.0 null null null null)
  (`/Game/Alexis_Garrigue/BP_AG_GameMaster.Subtitles` _gamemaster "Il est de ton devoir de construire ce mur,")
  (`KismetSystemLibrary.Delay` 2.0)
  (`/Game/Alexis_Garrigue/BP_AG_GameMaster.Subtitles` _gamemaster "tu récupéreras sûrement un fragment de blason.")
  (`KismetSystemLibrary.Delay` 4.0)
  (`/Game/Alexis_Garrigue/BP_AG_GameMaster.Subtitles` _gamemaster "")
  (`KismetSystemLibrary.Delay` 1.0)
  (`GameplayStatics.PlaySoundAtLocation` "/Game/Alexis_Garrigue/Dialogues/A_UtilisesMarteau.A_UtilisesMarteau" _returnvalue (struct) 1.0 1.0 0.0 null null null null)
  (`/Game/Alexis_Garrigue/BP_AG_GameMaster.Subtitles` _gamemaster "Utilises ce marteau pour détruire la maison et construire le mur avec les débris.")
  (`KismetSystemLibrary.Delay` 5.0)
  (`/Game/Alexis_Garrigue/BP_AG_GameMaster.Subtitles` _gamemaster "")
  (`/Game/Alexis_Garrigue/BP_AG_GameMaster.Quest` (`self.GameMaster`) "- Prends le marteau et casses la maison jaune."))

(fn `MiniGame`
  (bind _wall (`self.Wall`))
  (`parent.MiniGame`)
  (`PrimitiveComponent.SetCollisionEnabled` (`/Game/Alexis_Garrigue/Wall/BP_AG_WallTrigger.Box` _wall) "QueryOnly")
  (`KismetArrayLibrary.Array_Clear` (`/Game/Alexis_Garrigue/Wall/BP_AG_WallTrigger.Placed` _wall))
  (`self.BeginningDialogue`))

(fn `UserConstructionScript`
  (`parent.UserConstructionScript`))