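; Game master Blueprint that changes a tree's size and toggles the visibility of a set of point actors.
; ChangeTree plays a leaf-fall sound, swaps the static mesh by size index and spawns a Niagara tree-explosion effect on a newly added component.
; HideAll and ShowAll loop over AllPoints to hide or reveal each actor.
; The DialogueAndSubtitles event is an empty stub.
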(event `Dialogue And Subtitles`)

(fn `ChangeTree`
  (params (Size :type Integer))
  (`GameplayStatics.PlaySound2D` "/Game/Alexis_Garrigue/Sounds/LeavesFall.LeavesFall" 1.0 1.0 0.0 null null)
  (`StaticMeshComponent.SetStaticMesh` (`self.StaticMesh`) (`|GetArrayItem` (`self.TreeSizes`) Size))
  (bind _returnvalue (`AddComponent|NODE_AddNiagaraComponent-0`))
  (`NiagaraFunctionLibrary.SpawnSystemAttached` "/Game/Cesar/VFX/N_CVC_ExploArbre.N_CVC_ExploArbre" _returnvalue "bite" (0.0 -50.0 50.0) (struct) "KeepRelativeOffset"))

(fn `HideAll`
  (for _array_element (`self.AllPoints`)
    (`self.SetActorHiddenInGame` _array_element true)))

(fn `ShowAll`
  (for _array_element (`self.AllPoints`)
    (`self.SetActorHiddenInGame` _array_element false)))

(fn `UserConstructionScript`)