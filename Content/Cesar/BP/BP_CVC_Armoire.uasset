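; VR armoire Blueprint whose door swings while a motion controller holds it.
; Grab stores the controller if it is within the hand collision sphere's radius, and release clears it.
; Each tick, look-at yaw from controller to door, offset and clamped to a quarter turn, sets door rotation.
; When not held, the door snaps to zero world height if nearly there; the open-state check never runs.
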(event `self.ReceiveTick`
  (params (DeltaSeconds :type "Float (single-precision)"))
  (bind _motion_controler (`self.Motion Controler`))
  (bind _amoire (`self.amoire`))
  (bind (_returnvalue_x _returnvalue_y _returnvalue_z) (`KismetMathLibrary.BreakVector` (`SceneComponent.K2_GetComponentLocation` _amoire)))
  (bind (_returnvalue_x_2 _returnvalue_y_2) (`KismetMathLibrary.BreakVector` (`SceneComponent.K2_GetComponentLocation` (`self.amoire`))))
  (bind (_returnvalue_roll _returnvalue_pitch _returnvalue_yaw) (`KismetMathLibrary.BreakRotator` (`KismetMathLibrary.FindLookAtRotation` (`SceneComponent.K2_GetComponentLocation` _motion_controler) (`SceneComponent.K2_GetComponentLocation` _amoire))))
  ;[1 1 1] set door rotation
  (`/Engine/EditorBlueprintResources/StandardMacros.IsValid` _motion_controler
    (:`Is Valid`
      (`SceneComponent.K2_SetWorldRotation` (`self.amoire`) (`KismetMathLibrary.MakeRotator` 0.0 0.0 (`KismetMathLibrary.ClampAngle` (- _returnvalue_yaw 90.0) 0.0 90.0)) false false))
    (:`Is Not Valid`
      (if (`KismetMathLibrary.NearlyEqual_FloatFloat` _returnvalue_z 0.0 10.0)
        (`SceneComponent.K2_SetWorldLocation` _amoire (`KismetMathLibrary.MakeVector` _returnvalue_x_2 _returnvalue_y_2) false false)))))

(event `/Game/Cesar/BP/BP_CVC_Grab.realease`
  (params (MotionController :type "MotionControllerComponent Object Reference"))
  (if (== MotionController (`self.Motion Controler`))
    (set `self.Motion Controler` null)))

(event `/Game/Cesar/BP/BP_CVC_Grab.grab`
  (params (MotionControler :type "MotionControllerComponent Object Reference"))
  (bind _handcollide (`self.handcollide`))
  (if (== (`SceneComponent.K2_GetComponentLocation` MotionControler) (`SceneComponent.K2_GetComponentLocation` _handcollide) :`ErrorTolerance` (`SphereComponent.SphereRadius` _handcollide))
    (set `self.Motion Controler` MotionControler)
    (`KismetSystemLibrary.PrintString` "test 3")))

(fn `UserConstructionScript`)